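; PC_Puzzle_Controller is a player controller, apparently for a puzzle game, that handles test inputs with debug printing.
; BeginPlay casts and caches the PS_Player_Data player state, and the space bar action increments its PSHP and prints the value.
; Forward and Left actions only print their names.
; Disconnected nodes hold GM_Puzzle game mode logic for caching it, zeroing HP and triggering player death, which never runs.
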(event `self.ReceiveBeginPlay`
  (bind _asps_player_data (cast `/Game/Blueprints/PS_Player_Data` (`GameplayStatics.GetPlayerState` 0)))
  (set `self.As PS Player Data` _asps_player_data))

(event `InputAction|My_Space_bar`
  (params (Key :type "Key Structure"))
  (:`Pressed`
    (bind _output_get (set `/Game/Blueprints/PS_Player_Data.PS_HP` (+ (`/Game/Blueprints/PS_Player_Data.PS_HP` (`self.As PS Player Data`)) 1) (`self.As PS Player Data`)))
    (`KismetSystemLibrary.PrintString` (`KismetStringLibrary.Conv_IntToString` _output_get))))

(event `InputAction|My_Forward`
  (params (Key :type "Key Structure"))
  (:`Pressed`
    (`KismetSystemLibrary.PrintString` "Forward")))

(event `InputAction|My_Left`
  (params (Key :type "Key Structure"))
  (:`Pressed`
    (`KismetSystemLibrary.PrintString` "Left")))

(fn `UserConstructionScript`)